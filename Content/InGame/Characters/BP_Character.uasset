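; Playable character with targeted auto-attacks, six skill slots, inventory and an overhead HP bar.
; BeginPlay loads data-table stats, adds test items and pre-spawns a hidden arrow pool on the server.
; Attacks chase the target until in range, then repeat on an attack-speed timer, multicasting facing and montage, with PlayMontage left empty here.
; C2S events forward skills to SkillComponent, while update functions push HP, item and equipment state to the UI.
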(event `self.ReceiveBeginPlay`
  (`|ExecutionSequence`
    (:`then_0`
      (`self.InitializeStats`)
      (`self.HPBar`)
      (`self.ArrowSpawn`))
    (:`then_1`
      (`self.TestAddItem`)
      (`SkillComponent.SetTacticalSkill` (`self.SkillComponent`) (`self.TacticalSkillRowName`))
      (if (`self.IsLocallyControlled`)
        (bind _asbp_player_controller (cast `/Game/InGame/Player/BP_PlayerController` (`self.GetController`)))
        (`/Game/InGame/UI/HUD/BP_HUD.SetTacticalIcon` (`/Game/InGame/Player/BP_PlayerController.HUDRef` _asbp_player_controller) (`self.TacticalSkillRowName`))))))

(event `self.OnHPChanged`
  (params (InCurrentHP :type "Float (single-precision)") (InMaxHP :type "Float (single-precision)"))
  (`|ExecutionSequence`
    (:`then_0`
      (bind _aswbp_hpbar (cast `/Game/InGame/UI/PlayerWidgets/WBP_HPBar` (`WidgetComponent.GetWidget` (`self.HPBarWidget`))))
      (`ProgressBar.SetPercent` (`/Game/InGame/UI/PlayerWidgets/WBP_HPBar.HpBar` _aswbp_hpbar) (/ InCurrentHP InMaxHP)))
    (:`then_1`
      (if (`self.IsLocallyControlled`)
        (bind _asplayer_controller (cast `PlayerController` (`self.GetController`)))
        (bind _asbp_hud (cast `/Game/InGame/UI/HUD/BP_HUD` (`PlayerController.GetHUD` _asplayer_controller)))
        (`/Game/InGame/UI/HUD/BP_HUD.UpdateHP` _asbp_hud InCurrentHP InMaxHP)))))

(event `AttackTarget`
  (params (TargetActor :type "Actor Object Reference"))
  ; 기본 공격
  (set `self.bIsTargetInRange` false)
  (bind _output_get (set `self.TargetActor` TargetActor))
  (if (<= (`self.GetDistanceTo` _output_get) (+ (`CharacterStatComponent.GetFinalAttackRange` (`self.CharacterStatComponent`)) 100.0))
    (set `self.bIsTargetInRange` true)
    (`self.TryAttack` (`self.TargetActor`))
    (else
      (bind _asbp_player_controller (cast `/Game/InGame/Player/BP_PlayerController` (`self.GetController`)))
      (`EternalReturnPlayerController.RequestMoveTo` _asbp_player_controller (`self.K2_GetActorLocation` (`self.TargetActor`))))))

(event `self.AttackRangeSphere.OnComponentBeginOverlap`
  (params (OverlappedComponent :type "PrimitiveComponent Object Reference") (OtherActor :type "Actor Object Reference") (OtherComp :type "PrimitiveComponent Object Reference") (OtherBodyIndex :type Integer) (bFromSweep :type Boolean) (SweepResult :type "HitResult Structure (by ref)"))
  (bind _targetactor (`self.TargetActor`))
  ; 기본 공격
  (`/Engine/EditorBlueprintResources/ActorMacros.Switch Has Authority`
    (:`Authority`
      (if (and (== OtherActor _targetactor) (`KismetSystemLibrary.IsValid` _targetactor))
        (set `self.bIsTargetInRange` true)
        (`self.TryAttack` (`self.TargetActor`))))))

(event `self.AttackRangeSphere.OnComponentEndOverlap`
  (params (OverlappedComponent :type "PrimitiveComponent Object Reference") (OtherActor :type "Actor Object Reference") (OtherComp :type "PrimitiveComponent Object Reference") (OtherBodyIndex :type Integer))
  (bind _targetactor (`self.TargetActor`))
  ; 기본 공격
  (`/Engine/EditorBlueprintResources/ActorMacros.Switch Has Authority`
    (:`Authority`
      (if (and (== OtherActor _targetactor) (`KismetSystemLibrary.IsValid` _targetactor))
        (set `self.bIsTargetInRange` false)
        (bind _ascombat_entity_base (cast `CombatEntityBase` (`self.TargetActor`)))
        (if (not (`self.IsDead` _ascombat_entity_base))
          (bind _asbp_player_controller (cast `/Game/InGame/Player/BP_PlayerController` (`self.GetController`)))
          (`EternalReturnPlayerController.RequestMoveTo` _asbp_player_controller (`self.K2_GetActorLocation` (`self.TargetActor`))))))))

(event `S2M_AttackMontage`
  (`self.StopAnimMontage` "/Game/Assets/Rio/Animations/AM_RioAttack.AM_RioAttack")
  (`self.PlayMontage` (`CharacterStatComponent.GetFinalAttackSpeed` (`self.CharacterStatComponent`))))

(event `C2S_SkillQ`
  ; Skill
  (`SkillComponent.ExecuteSkill` (`self.SkillComponent`) "Skill_Q"))

(event `C2S_ClearTarget`
  (`self.ClearTarget`))

(event `C2S_SkillW`
  ; Skill
  (`SkillComponent.ExecuteSkill` (`self.SkillComponent`) "Skill_W"))

(event `C2S_SkillE`
  ; Skill
  (`SkillComponent.ExecuteSkill` (`self.SkillComponent`) "Skill_E"))

(event `S2M_SetRotation`
  (params (NewYaw :type "Float (double-precision)"))
  (`self.K2_SetActorRotation` (`KismetMathLibrary.MakeRotator` 0.0 0.0 NewYaw)))

(event `C2S_SkillR`
  ; Skill
  (`SkillComponent.ExecuteSkill` (`self.SkillComponent`) "Skill_R"))

(event `C2S_SkillD`
  ; Skill
  (`SkillComponent.ExecuteSkill` (`self.SkillComponent`) "Skill_D"))

(event `C2S_SkillF`
  ; Skill
  (`SkillComponent.ExecuteSkill` (`self.SkillComponent`) "Skill_F"))

(fn `ArrowSpawn`
  (locals (spawnindex :type Integer :default 6))
  (`/Engine/EditorBlueprintResources/ActorMacros.Switch Has Authority`
    (:`Authority`
      (for _ (range (+ (`local.spawnindex`) 1))
        (bind _returnvalue (`|SpawnActorFromClass` "/Game/InGame/Characters/Subject/BP_Arrow.BP_Arrow_C" (`KismetMathLibrary.MakeTransform` (`self.K2_GetActorLocation` self)) "Undefined" "MultiplyWithRoot" null null))
        (`KismetArrayLibrary.Array_Add` (`self.ArrowArray`) _returnvalue)
        (`self.SetActorHiddenInGame` _returnvalue true)
        (`PrimitiveComponent.SetCollisionEnabled` (`/Game/InGame/Characters/Subject/BP_Arrow.Sphere` _returnvalue) "NoCollision")))))

(fn `CameraSet`)

(fn `ClearTarget`
  (set `self.TargetActor` null)
  (set `self.bIsTargetInRange` false)
  (set `self.bIsCanAttack` true)
  (`KismetSystemLibrary.K2_ClearTimer` null "OnAttackCooldownEnd"))

(fn `EquipSlotsUpdate`
  (bind _hudref (`self.HUDRef`))
  (`/Engine/EditorBlueprintResources/StandardMacros.IsValid` _hudref
    (:`Is Valid`
      (for _index (range 5)
        (`/Game/InGame/UI/PlayerWidgets/WBP_ItemUI.SetItem` (`|GetArrayItem` (`/Game/InGame/UI/PlayerWidgets/WBP_HUD.EquipSlotWidgets` (`/Game/InGame/UI/HUD/BP_HUD.MainUIRef` _hudref)) _index) (`.ItemID` (break `InventorySlot` (`|GetArrayItem` (`InventoryComponent.EquipSlots` (`self.InventoryComponent`)) _index))))))))

(fn `HPBar`
  (locals (HPBarRef :type "/Game/InGame/UI/PlayerWidgets/WBP_HPBar Object Reference"))
  (bind _aswbp_hpbar (cast `/Game/InGame/UI/PlayerWidgets/WBP_HPBar` (`WidgetComponent.GetUserWidgetObject` (`self.HPBarWidget`))))
  (bind _output_get (set `local.HPBarRef` _aswbp_hpbar))
  (`TextBlock.SetText` (`/Game/InGame/UI/PlayerWidgets/WBP_HPBar.NameText` _output_get) (`KismetTextLibrary.Conv_NameToText` (`self.CharacterRowName`)))
  (if (`self.IsLocallyControlled`)
    (`ProgressBar.SetFillColorAndOpacity` (`/Game/InGame/UI/PlayerWidgets/WBP_HPBar.HpBar` _output_get) (struct :`G` 1.0 :`A` 1.0))
    (else
      (`ProgressBar.SetFillColorAndOpacity` (`/Game/InGame/UI/PlayerWidgets/WBP_HPBar.HpBar` _output_get) (struct :`R` 1.0 :`A` 1.0)))))

(fn `InitializeStats`
  (bind _returnvalue (`|GetDataTableRow` "/Game/InGame/Data/Tables/DT_CharacterData.DT_CharacterData" (`self.CharacterRowName`))
    (:`then`
      (`|ExecutionSequence`
        (:`then_0`
          (bind (_charactername _maxhp _hpregen _attackpower _defense _movespeed _attackspeed _attackrange _allowedweapontype) (break `/Game/InGame/Data/Structs/S_CharacterTableRow` _returnvalue))
          (`self.SetMaxHP` _maxhp)
          (`self.SetHPRegen` _hpregen))
        (:`then_1`
          (`self.SetAttackPower` _attackpower)
          (`self.SetAttackSpeed` _attackspeed)
          (`self.SetAttackRange` _attackrange))
        (:`then_2`
          (`self.SetDefense` _defense)
          (`self.SetMoveSpeed` _movespeed))
        (:`then_3`
          (set `self.AllowedWeaponType` _allowedweapontype))
        (:`then_4`
          (bind _asbp_player_controller (cast `/Game/InGame/Player/BP_PlayerController` (`self.GetController`)))
          (bind _asbp_hud (cast `/Game/InGame/UI/HUD/BP_HUD` (`PlayerController.GetHUD` _asbp_player_controller)))
          (`/Game/InGame/UI/PlayerWidgets/WBP_HUD.UpdateStatUI` (`/Game/InGame/UI/HUD/BP_HUD.MainUIRef` _asbp_hud)))))
    (:`RowNotFound`
      (`KismetSystemLibrary.PrintString` "Character Data Not Found" true true (struct :`G` 0.66 :`B` 1.0 :`A` 1.0) 99999.0))))

(fn `InventorySlotsUpdate`
  (bind _hudref (`self.HUDRef`))
  (`KismetSystemLibrary.PrintString` "InventorySlotsUpdate 호출됨")
  (`/Engine/EditorBlueprintResources/StandardMacros.IsValid` _hudref
    (:`Is Valid`
      (for _index (range 10)
        (`/Game/InGame/UI/PlayerWidgets/WBP_ItemUI.SetItem` (`|GetArrayItem` (`/Game/InGame/UI/PlayerWidgets/WBP_HUD.InventorySlotWidgets` (`/Game/InGame/UI/HUD/BP_HUD.MainUIRef` _hudref)) _index) (`.ItemID` (break `InventorySlot` (`|GetArrayItem` (`InventoryComponent.InventorySlots` (`self.InventoryComponent`)) _index))))))
    (:`Is Not Valid`
      (`KismetSystemLibrary.PrintString` "HUDRef가 null임"))))

(fn `MouseDown`)

(fn `MouseLeft`)

(fn `MouseRight`)

(fn `MouseUp`)

(fn `OnAttackCooldownEnd`
  (set `self.bIsCanAttack` true)
  (`self.TryAttack` (`self.TargetActor`)))

(fn `PlayMontage`
  (params (AttackSpeed :type "Float (double-precision)")))

(fn `TestAddItem`
  (if (`self.HasAuthority`)
    (`InventoryComponent.AddItem` (`self.InventoryComponent`) "Bow_006_MightyBow")
    (`InventoryComponent.AddItem` (`self.InventoryComponent`) "Mat_Feather")
    (`InventoryComponent.AddItem` (`self.InventoryComponent`) "Arm_051_DiceOfDestiny")
    (`InventoryComponent.AddItem` (`self.InventoryComponent`) "Chest_046_BloodCloak")
    (`InventoryComponent.AddItem` (`self.InventoryComponent`) "Head_035_FallenPegasus")
    (`InventoryComponent.AddItem` (`self.InventoryComponent`) "Leg_033_Alexander")))

(fn `TryAttack`
  (params (Target :type "Actor Object Reference"))
  (bind _ascombat_entity_base (cast `CombatEntityBase` Target))
  (if (and (`KismetSystemLibrary.IsValid` Target) (`self.bIsCanAttack`) (`self.bIsTargetInRange`) (not (`self.IsDead` _ascombat_entity_base)) (not (`self.IsDead`)))
    (set `self.bIsCanAttack` false)
    (bind (_returnvalue_roll _returnvalue_pitch _returnvalue_yaw) (`KismetMathLibrary.BreakRotator` (`KismetMathLibrary.FindLookAtRotation` (`self.K2_GetActorLocation` self) (`self.K2_GetActorLocation` _ascombat_entity_base))))
    (`self.S2M_SetRotation` _returnvalue_yaw)
    (bind _asbp_player_controller (cast `/Game/InGame/Player/BP_PlayerController` (`self.GetController`)))
    (`EternalReturnPlayerController.StopPathFollowing` _asbp_player_controller)
    (`self.S2M_AttackMontage`)
    (`KismetSystemLibrary.K2_SetTimer` null "OnAttackCooldownEnd" (/ 1.0 (`CharacterStatComponent.GetFinalAttackSpeed` (`self.CharacterStatComponent`))))))

(fn `UserConstructionScript`)