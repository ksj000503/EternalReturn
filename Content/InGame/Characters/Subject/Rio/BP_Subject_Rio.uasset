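; BP_Subject_Rio is the Blueprint for Rio, a Subject character that attacks by shooting arrows at a target.
; C2S_ShootArrow, named as a client-to-server event, activates the first inactive arrow in a pooled array, passing the target, stat-derived damage and attack-speed-scaled projectile speed.
; PlayMontage swaps to a faster triple-attack montage while the skill toggle is on, using fixed play rates that ignore its AttackSpeed input.
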(event `C2S_ShootArrow`
  (for _array_element (`self.ArrowArray`)
    (if (not (`/Game/InGame/Characters/Subject/Rio/BP_Arrow.bIsActive` _array_element))
      (`/Game/InGame/Characters/Subject/Rio/BP_Arrow.Activate` _array_element (`self.TargetActor`) (`CharacterStatComponent.GetFinalAttackPower` (`self.CharacterStatComponent`)) (* (`BaseStatComponent.GetAttackSpeed` (`self.StatComponent`)) 1000.0) (`self.K2_GetActorLocation`) self)
      (break))))

(fn `PlayMontage`
  (params (AttackSpeed :type "Float (double-precision)"))
  (`parent.PlayMontage` 0.0)
  (if (`SkillComponent.bUseToggle` (`self.SkillComponent`))
    (`self.PlayAnimMontage` "/Game/Assets/Rio/Animations/AM_RioTripleAttack.AM_RioTripleAttack" 3.0)
    (else
      (`self.PlayAnimMontage` "/Game/Assets/Rio/Animations/AM_RioAttack.AM_RioAttack"))))

(fn `UserConstructionScript`
  (`parent.UserConstructionScript`))