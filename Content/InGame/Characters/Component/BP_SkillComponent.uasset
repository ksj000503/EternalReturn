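; Character skill component for Q/W/E/R/D/F skills and a tactical skill, largely unfinished: skill handlers except Toggle are empty.
; Cooldowns use per-key timers, but one shared KeyType lets overlapping skills clear the wrong handle, noted for a C++ fix.
; ExecuteSkill's cooldown check and dispatch by key and skill type are disconnected, as is the tactical DataTable lookup.
; SetTacticalSkill only stores the row name; UseTacticalSkill routes to an empty Blink.
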(event `self.ReceiveTick`
  (params (DeltaSeconds :type "Float (single-precision)")))

(event `OnSkillExecuted`
  (params (KeyType :type "/Game/InGame/Data/Enum/E_SkillKeyType Enum" :default "NewEnumerator0") (Cooldown :type "Float (double-precision)"))
  (set `self.Key Type` KeyType)
  (bind _returnvalue (`KismetSystemLibrary.K2_SetTimerDelegate` (delegate `OnCooldownFinished`) Cooldown))
  (`BlueprintMapLibrary.Map_Add` (`self.TimeHandle`) KeyType _returnvalue))

(event `OnCooldownFinished`
  (`KismetSystemLibrary.K2_ClearAndInvalidateTimerHandle` (`BlueprintMapLibrary.Map_Find` (`self.TimeHandle`) (`self.Key Type`)))
  (`BlueprintMapLibrary.Map_Add` (`self.SkillCooldown`) (`self.Key Type`)))

(fn `AreaDamage `)

(fn `Blink`)

(fn `Buff`)

(fn `CC`)

(fn `Dash`)

(fn `ExecuteSkill`
  (params (KeyType :type "/Game/InGame/Data/Enum/E_SkillKeyType Enum" :default "NewEnumerator0")))

(fn `Passive`)

(fn `Projectile`)

(fn `SetTacticalSkill`
  (params (NewParam :type Name))
  (returns (Output_Get :type "FallbackStruct Structure"))
  (set `self.RowName` NewParam))

(fn `SkillType`
  (params (Selection :type "/Game/InGame/Data/Enum/E_SkillType Enum" :default "NewEnumerator0") (SkillData :type "Object Object Reference"))
  (switch `/Game/InGame/Data/Enum/E_SkillType` Selection
    (:`NewEnumerator0`
      (`self.Passive`))
    (:`NewEnumerator1`
      (`self.Toggle`))
    (:`NewEnumerator2`
      (`self.Buff`))
    (:`NewEnumerator3`
      (`self.Projectile`))
    (:`NewEnumerator4`
      (`self.Dash`))
    (:`NewEnumerator5`
      (`self.CC`))
    (:`NewEnumerator6`
      (`self.AreaDamage `))))

(fn `Toggle`
  (if (`self.bUseToggle`)
    (set `self.bUseToggle` false)
    (else
      (set `self.bUseToggle` true))))

(fn `UpdateCooldown`
  (params (DeltaTime :type "Float (double-precision)") (KeyType :type "/Game/InGame/Data/Enum/E_SkillKeyType Enum" :default "NewEnumerator0")))

(fn `UseTacticalSkill`
  (params (NewParam :type Byte :default 0))
  (switch `|SwitchEnum` (`.SkillType_10_453209934FFDC3A22FE26FA80FE1A46D` (break `FallbackStruct` (`self.TaticalSkill`)))
    (:`NewEnumerator0`
      (`self.Blink`))))