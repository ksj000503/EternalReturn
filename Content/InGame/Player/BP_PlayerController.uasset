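; BP_PlayerController is the player controller that turns click events into commands for the possessed BP_Character.
; On possess, it hands its BP_HUD to the character as HUDRef.
; A ground click calls C2SClearTarget on the character, and an enemy click passes that actor to AttackTarget.
; A structure click only stores the BP_StructureBase as TargetStructure and sets an interact flag, which this graph never consumes.
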(event `self.ReceivePossess`
  (params (PossessedPawn :type "Pawn Object Reference"))
  (bind _asbp_character (cast `/Game/InGame/Characters/BP_Character` PossessedPawn))
  (bind _asbp_hud (cast `/Game/InGame/UI/HUD/BP_HUD` (`self.GetHUD`)))
  (set `/Game/InGame/Characters/BP_Character.HUDRef` _asbp_hud _asbp_character))

(event `self.OnGroundClicked`
  (bind _asbp_character (cast `/Game/InGame/Characters/BP_Character` (`self.K2_GetPawn`)))
  (`/Game/InGame/Characters/BP_Character.C2S_ClearTarget` _asbp_character))

(event `self.OnEnemyClicked`
  (params (EnemyActor :type "Actor Object Reference"))
  (bind _asbp_character (cast `/Game/InGame/Characters/BP_Character` (`self.K2_GetPawn`)))
  (`/Game/InGame/Characters/BP_Character.AttackTarget` _asbp_character EnemyActor))

(event `self.OnStructureClicked`
  (params (StructureActor :type "Actor Object Reference"))
  (bind _asbp_structure_base (cast `/Game/InGame/World/Structures/BP_StructureBase` StructureActor))
  (set `self.TargetStructure ` _asbp_structure_base)
  (set `self.bIsWantsToInteract ` true))

(fn `UserConstructionScript`)