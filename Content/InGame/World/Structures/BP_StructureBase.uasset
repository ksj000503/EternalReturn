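; BP_StructureBase is a base for world structures that open a structure UI and replicate an item list.
; When a character overlaps its Box and its controller wants to interact, it passes StructureID to the HUD and clears the interact flag.
; On remote machines, the ItemList RepNotify scans all player controllers and reinitializes slots on any valid LootBoxRef that equals that controller's TargetStructure.
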(event `self.Box.OnComponentBeginOverlap`
  (params (OverlappedComponent :type "PrimitiveComponent Object Reference") (OtherActor :type "Actor Object Reference") (OtherComp :type "PrimitiveComponent Object Reference") (OtherBodyIndex :type Integer) (bFromSweep :type Boolean) (SweepResult :type "HitResult Structure (by ref)"))
  (bind _asbp_character (cast `/Game/InGame/Characters/BP_Character` OtherActor))
  (bind _asbp_player_controller (cast `/Game/InGame/Player/BP_PlayerController` (`Pawn.GetController` _asbp_character)))
  (if (`/Game/InGame/Player/BP_PlayerController.bIsWantsToInteract ` _asbp_player_controller)
    (bind _asbp_hud (cast `/Game/InGame/UI/HUD/BP_HUD` (`PlayerController.GetHUD` _asbp_player_controller)))
    (`/Game/InGame/UI/HUD/BP_HUD.StructureUI` _asbp_hud (`self.StructureID`))
    (set `/Game/InGame/Player/BP_PlayerController.bIsWantsToInteract ` false _asbp_player_controller)))

(fn `OnRep_ItemList`
  (`/Engine/EditorBlueprintResources/ActorMacros.Switch Has Authority`
    (:`Remote`
      (bind _outactors (`GameplayStatics.GetAllActorsOfClass` "/Game/InGame/Player/BP_PlayerController.BP_PlayerController_C"))
      (for _array_element _outactors
        (bind _lootboxref (`/Game/InGame/Player/BP_PlayerController.LootBoxRef` _array_element))
        (`/Engine/EditorBlueprintResources/StandardMacros.IsValid` _lootboxref
          (:`Is Valid`
            (if (== _lootboxref (`/Game/InGame/Player/BP_PlayerController.TargetStructure ` _array_element))
              (`/Game/InGame/UI/LootWidgets/WBP_LootBox.InitSlots` _lootboxref (`self.ItemList`)))))))))

(fn `UserConstructionScript`)