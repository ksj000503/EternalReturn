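; BP_MonsterBase is the base monster Blueprint, setting up a monster's stats and health bar display.
; On BeginPlay it fills health, combat, movement and drop values from the DT_MonsterData row named by MonsterRowName, then colors the WBP_HPBar widget red.
; OnHPChanged updates the bar's percent from current over max HP.
; The DropGold value is written into DropExp and immediately overwritten, so gold is not kept.
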(event `self.ReceiveBeginPlay`
  (`self.InitializeStats`)
  (`self.HPBar`))

(event `self.OnHPChanged`
  (params (InCurrentHP :type "Float (single-precision)") (InMaxHP :type "Float (single-precision)"))
  (bind _aswbp_hpbar (cast `/Game/InGame/UI/Widgets/WBP_HPBar` (`WidgetComponent.GetWidget` (`self.HPBarWidget`))))
  (`ProgressBar.SetPercent` (`/Game/InGame/UI/Widgets/WBP_HPBar.HpBar` _aswbp_hpbar) (/ InCurrentHP InMaxHP)))

(fn `HPBar`
  (locals (HPBarRef :type "/Game/InGame/UI/Widgets/WBP_HPBar Object Reference"))
  (bind _aswbp_hpbar (cast `/Game/InGame/UI/Widgets/WBP_HPBar` (`WidgetComponent.GetUserWidgetObject` (`self.HPBarWidget`))))
  (bind _output_get (set `local.HPBarRef` _aswbp_hpbar))
  (`ProgressBar.SetFillColorAndOpacity` (`/Game/InGame/UI/Widgets/WBP_HPBar.HpBar` _output_get) (struct :`R` 1.0 :`A` 1.0)))

(fn `InitializeStats`
  (bind _returnvalue (`|GetDataTableRow` "/Game/InGame/Data/Tables/DT_MonsterData.DT_MonsterData" (`self.MonsterRowName`))
    (:`then`
      (`|ExecutionSequence`
        (:`then_0`
          (bind (_monstername _maxhp _attackpower _defense _movespeed _attackspeed _attackrange _dropgold _dropexp) (break `/Game/InGame/Data/Structs/S_MonsterTableRow` _returnvalue))
          (`self.SetMaxHP` _maxhp))
        (:`then_1`
          (`self.SetAttackPower` _attackpower)
          (`self.SetAttackSpeed` _attackspeed)
          (`self.SetAttackRange` _attackrange))
        (:`then_2`
          (`self.SetDefense` _defense)
          (`self.SetMoveSpeed` _movespeed))
        (:`then_3`
          (set `self.DropExp` _dropgold)
          (set `self.DropExp` _dropexp))))))

(fn `UserConstructionScript`)