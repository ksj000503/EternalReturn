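; BP_Arrow is a reusable homing projectile that damages a single assigned target.
; Activate stores target, damage, speed and causer, moves it to the shoot location and enables its sphere overlap.
; Tick steers it straight at the target's current location without sweeping, deactivating if the target becomes invalid.
; On overlap with that target, only the authority applies damage and calls Deactivate, which hides and disables the arrow for reuse instead of destroying it.
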(event `self.ReceiveTick`
  (params (DeltaSeconds :type "Float (single-precision)"))
  (if (`self.bIsActive`)
    (`/Engine/EditorBlueprintResources/StandardMacros.IsValid` (`self.Target Actor`)
      (:`Is Valid`
        (`self.K2_AddActorWorldOffset` (* (`self.Speed`) DeltaSeconds (`KismetMathLibrary.Normal` (- (`self.K2_GetActorLocation` (`self.Target Actor`)) (`self.K2_GetActorLocation`))))))
      (:`Is Not Valid`
        (`self.Deactivate`)))))

(event `self.Sphere.OnComponentBeginOverlap`
  (params (OverlappedComponent :type "PrimitiveComponent Object Reference") (OtherActor :type "Actor Object Reference") (OtherComp :type "PrimitiveComponent Object Reference") (OtherBodyIndex :type Integer) (bFromSweep :type Boolean) (SweepResult :type "HitResult Structure (by ref)"))
  (`/Engine/EditorBlueprintResources/ActorMacros.Switch Has Authority`
    (:`Authority`
      (if (== OtherActor (`self.Target Actor`))
        (`GameplayStatics.ApplyDamage` (`self.Target Actor`) (`self.Damage`) null (`self.DamageCauser`))
        (`self.Deactivate`)))))

(fn `Activate`
  (params (TargetActor :type "Actor Object Reference") (Damage :type "Float (double-precision)") (Speed :type "Float (double-precision)") (ShootLocation :type "Vector Structure") (DamageCauser :type "Actor Object Reference"))
  (set `self.Target Actor` TargetActor)
  (set `self.Damage` Damage)
  (set `self.Speed` Speed)
  (set `self.DamageCauser` DamageCauser)
  (`self.K2_SetActorLocation` ShootLocation)
  (`self.SetActorHiddenInGame` false)
  (`PrimitiveComponent.SetCollisionEnabled` (`self.Sphere`) "QueryOnly")
  (set `self.bIsActive` true))

(fn `Deactivate`
  (`self.SetActorHiddenInGame` true)
  (`PrimitiveComponent.SetCollisionEnabled` (`self.Sphere`) "NoCollision")
  (set `self.bIsActive` false)
  (set `self.Target Actor` null))

(fn `UserConstructionScript`)