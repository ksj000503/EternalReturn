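; BP_LobbyGS is the lobby game state, holding a DelayTime value that is shown on each client's lobby UI.
; When DelayTime replicates, its OnRep runs only on the remote side, going from the local BP_LobbyPC through BP_LobbyHud to LobbymainUI to call UpdateTime.
; BeginPlay, Tick and the construction script are empty, and a few leftover nodes never run.
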(event `self.ReceiveBeginPlay`)

(fn `OnRep_DelayTime`
  (`/Engine/EditorBlueprintResources/ActorMacros.Switch Has Authority`
    (:`Remote`
      (bind _asbp_lobby_pc (cast `/Game/Lobby/Player/BP_LobbyPC` (`GameplayStatics.GetPlayerController` 0)))
      (bind _asbp_lobby_hud (cast `/Game/Lobby/UI/HUD/BP_LobbyHud` (`PlayerController.GetHUD` _asbp_lobby_pc)))
      (set `self.Lobbymain UI` (`/Game/Lobby/UI/HUD/BP_LobbyHud.LobbymainUI` _asbp_lobby_hud))
      (`/Game/Lobby/UI/Widget/WBP_LobbyMainUI.UpdateTime` (`self.Lobbymain UI`) (`self.DelayTime`)))))

(fn `UserConstructionScript`)