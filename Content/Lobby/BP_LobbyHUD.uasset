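; BP_LobbyHUD is the lobby HUD that puts the lobby and room UI widgets on screen.
; On BeginPlay it creates WBP_LobbyUI and WBP_Room for the first player controller and adds both to the viewport.
; The room widget is stored in RoomRef and starts hidden, and the RoomOn function makes it visible without hiding the lobby UI.
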(event `self.ReceiveBeginPlay`
  (bind _returnvalue (`|CreateWidget` "/Game/Lobby/UI/WBP_LobbyUI.WBP_LobbyUI_C" (`GameplayStatics.GetPlayerController` 0)))
  (`UserWidget.AddToViewport` _returnvalue 0)
  (bind _returnvalue_2 (`|CreateWidget` "/Game/Lobby/UI/WBP_Room.WBP_Room_C" (`GameplayStatics.GetPlayerController` 0)))
  (bind _output_get (set `self.RoomRef` _returnvalue_2))
  (`UserWidget.AddToViewport` _output_get 0)
  (`Widget.SetVisibility` _output_get "Hidden"))

(fn `RoomOn`
  (`Widget.SetVisibility` (`self.RoomRef`) "Visible"))

(fn `UserConstructionScript`)