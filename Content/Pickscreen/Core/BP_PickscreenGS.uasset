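; Game state for the pick screen, replicating a DelayTime value to display in the lobby UI.
; The DelayTime RepNotify gets the first player controller's HUD, takes its main lobby widget and passes the new time to its UpdateTime.
; Nothing in this graph sets or counts the time; BeginPlay and Tick are empty, and leftover authority, validity and player-array nodes never run.
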(event `self.ReceiveBeginPlay`)

(fn `OnRep_DelayTime`
  (bind _asbp_pickscreen_pc (cast `/Game/Pickscreen/Player/BP_PickscreenPC` (`GameplayStatics.GetPlayerController` 0)))
  (bind _asbp_pickscreen_hud (cast `/Game/Pickscreen/UI/HUD/BP_PickscreenHud` (`PlayerController.GetHUD` _asbp_pickscreen_pc)))
  (set `self.Lobbymain UI` (`/Game/Pickscreen/UI/HUD/BP_PickscreenHud.LobbymainUI` _asbp_pickscreen_hud))
  (`/Game/Pickscreen/UI/Widget/WBP_LobbyMainUI.UpdateTime` (`self.Lobbymain UI`) (`self.DelayTime`)))

(fn `UserConstructionScript`)