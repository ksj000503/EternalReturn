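; Game mode for the pick screen that counts down and then moves the match to TestMap.
; A looping one-second timer decrements the clamped DelayTime on BP_PickscreenGS.
; At zero, it checks each tick that every BP_PlayerState has a SelectName other than "None".
; Once all have selected, it waits briefly and runs a ServerTravel console command, guarded by a flag against repeat transitions.
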(event `self.ReceiveBeginPlay`
  (`KismetSystemLibrary.K2_SetTimerDelegate` (delegate `Timer`) 1.0 true))

(event `Timer`
  (bind _asbp_pickscreen_gs (cast `/Game/Pickscreen/Core/BP_PickscreenGS` (`GameplayStatics.GetGameState`)))
  (bind _result (`/Engine/EditorBlueprintResources/StandardMacros.DecrementInt` (`/Game/Pickscreen/Core/BP_PickscreenGS.DelayTime` _asbp_pickscreen_gs))
    (:`  `
      (bind _output_get (set `/Game/Pickscreen/Core/BP_PickscreenGS.DelayTime` (`KismetMathLibrary.Clamp` _result 0 40) _asbp_pickscreen_gs))
      (if (== _output_get 0)
        (bind _bisallready (`self.AreAllPlayersReady`))
        (if _bisallready
          (`KismetSystemLibrary.Delay` 1.0)
          (if (not (`self.bHasStartedTransition `))
            (set `self.bHasStartedTransition ` true)
            (`KismetSystemLibrary.ExecuteConsoleCommand` "ServerTravel /Game/Maps/TestMap" null)))))))

(fn `AreAllPlayersReady`
  (returns (bIsAllReady :type Boolean))
  (locals (AllSelected :type Boolean))
  (for _array_element (`GameStateBase.PlayerArray` (`GameplayStatics.GetGameState`))
    (bind _asbp_player_state (cast `/Game/Pickscreen/Player/BP_PlayerState` _array_element))
    (if (== (`/Game/Pickscreen/Player/BP_PlayerState.SelectName` _asbp_player_state) "None")
      (set `local.AllSelected` false)
      (break)
      (else
        (set `local.AllSelected` true))))
  (return (`local.AllSelected`)))

(fn `UserConstructionScript`)