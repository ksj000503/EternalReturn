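; BP_LoginHUD sets up the login screen, showing the login UI and preparing a hidden signup panel.
; On BeginPlay it sets UI-only input for the first player controller and adds WBP_LoginUI and WBP_Signup to the viewport.
; It stores the signup widget and hides it until the SignUp function makes it visible.
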(event `self.ReceiveBeginPlay`
  (`WidgetBlueprintLibrary.SetInputMode_UIOnlyEx` (`GameplayStatics.GetPlayerController` 0) null)
  (bind _returnvalue (`|CreateWidget` "/Game/Login/UI/WBP_LoginUI.WBP_LoginUI_C"))
  (`UserWidget.AddToViewport` _returnvalue 0)
  (bind _returnvalue_2 (`|CreateWidget` "/Game/Login/UI/WBP_Signup.WBP_Signup_C"))
  (`UserWidget.AddToViewport` _returnvalue_2 0)
  (set `self.SignupRef` _returnvalue_2)
  (`Widget.SetVisibility` _returnvalue_2 "Hidden"))

(fn `SignUp`
  (`Widget.SetVisibility` (`self.SignupRef`) "Visible"))

(fn `UserConstructionScript`)